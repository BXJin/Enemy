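; BP_Zombie is the enemy zombie character, with a melee attack against the third-person player character.
; An AttackCapsule overlap sets a Blackboard flag for the AI's behavior logic, cleared after a short delay when the player leaves.
; AttackPlayer plays an attack montage and immediately sphere-traces ahead, applying damage if it hits the player.
; UpdateChaseSpeed sets walk speed; the PawnSensing see-pawn event is empty.
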(event OnSeePawn(PawnSensing)
  (params (Pawn :type Pawn%20Object%20Reference)))

(event OnComponentBeginOverlap(AttackCapsule)
  (params (OverlappedComponent :type Primitive%20Component%20Object%20Reference) (OtherActor :type Actor%20Object%20Reference) (OtherComp :type Primitive%20Component%20Object%20Reference) (OtherBodyIndex :type Integer) (bFromSweep :type Boolean) (SweepResult :type Hit%20Result%20Structure%20%28by%20ref%29))
  (Utilities|Casting|CastToBP_ThirdPersonCharacter OtherActor)
  (AI|Components|Blackboard|SetValueasBool (AI|GetBlackboard (AI|GetAIController self)) (Utilities|Name|MakeLiteralName "IsPlayerOverlap?") true))

(event OnComponentEndOverlap(AttackCapsule)
  (params (OverlappedComponent :type Primitive%20Component%20Object%20Reference) (OtherActor :type Actor%20Object%20Reference) (OtherComp :type Primitive%20Component%20Object%20Reference) (OtherBodyIndex :type Integer))
  (Utilities|Casting|CastToBP_ThirdPersonCharacter OtherActor)
  (Utilities|FlowControl|Delay 0.5)
  (AI|Components|Blackboard|SetValueasBool (AI|GetBlackboard (AI|GetAIController self)) (Utilities|Name|MakeLiteralName "IsPlayerOverlap?") false))

(event Custom|AttackPlayer
  (bind _returnvalue (Transformation|GetActorRotation))
  (bind _returnvalue_2 (Transformation|GetActorLocation))
  (bind _returnvalue_3 (Math|Vector|GetForwardVector _returnvalue))
  (Animation|PlayAnimMontage "/Game/Zombie/Animation/Zombie_Attack_Montage.Zombie_Attack_Montage" 1.5 "None")
  (bind (_outhit _returnvalue_4) (Collision|SphereTraceForObjects (+ _returnvalue_2 (* _returnvalue_3 1e+02)) (+ _returnvalue_2 (* _returnvalue_3 1.7e+02)) 3e+01 (Utilities|Array|MakeArray "ObjectTypeQuery3") false 0 "ForDuration"))
  (if _returnvalue_4
    (Utilities|Casting|CastToBP_ThirdPersonCharacter (.HitActor (Collision|BreakHitResult _outhit)))
    (Game|Damage|ApplyDamage (.HitActor (Collision|BreakHitResult _outhit)) 1e+01 0 0)))

(fn ConstructionScript)

(fn UpdateChaseSpeed
  (params (Speed :type Float%20%28double-precision%29))
  (Variables|/Script/Engine.CharacterMovementComponent|SetMaxWalkSpeed (Variables|Character|GetCharacterMovement) Speed))