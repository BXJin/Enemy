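; BP_Enemy is a zombie enemy that chases a player pawn, picked by ChaseIndex from BP_GM's controller list, and melees it.
; ChasePlayer uses AIMoveTo, then Attack faces the target and plays a montage, repeating or resuming the chase by distance.
; AttackTrace, meant for an AnimNotify, sphere-traces ahead to damage BP_ThirdPersonCharacter.
; GetDamage reduces Health and destroys the enemy at zero; BeginPlay does not start the chase.
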(event Custom|ChasePlayer
  ;[1 1 1] 플레이어 쫓기
  (Utilities|IsValid (Variables|Default|GetChaseChar)
    (:Is%20Valid
      _)
    (:Is%20Not%20Valid
      (CallFunction|SetChar)))
  (AI|AIMoveTo self "0, 0, 0" (Variables|Default|GetChaseChar) 1e+02 false
    (:OnSuccess
      (CallFunction|Attack))))

(event Custom|Attack
  ;[1 1 1] 플레이어 공격
  (Transformation|SetActorRotation (Math|Rotator|FindLookatRotation (Transformation|GetActorLocation self) (Transformation|GetActorLocation (Variables|Default|GetChaseChar))))
  (CallFunction|PlayAttackMontange))

(event Custom|AttackTrace
  (bind _returnvalue (Transformation|GetActorRotation))
  (bind _returnvalue_2 (Transformation|GetActorLocation))
  (bind _returnvalue_3 (Math|Vector|GetForwardVector _returnvalue))
  ;[1 1 1] AnimNotify로 불러올 함수내용
  (bind (_outhit _returnvalue_4) (Collision|SphereTraceForObjects (+ _returnvalue_2 (* _returnvalue_3 1e+02)) (+ _returnvalue_2 (* _returnvalue_3 1.7e+02)) 3e+01 (Utilities|Array|MakeArray "ObjectTypeQuery3") false 0 "ForDuration"))
  (if _returnvalue_4
    (bind _asbp_third_person_character (Utilities|Casting|CastToBP_ThirdPersonCharacter (.HitActor (Collision|BreakHitResult _outhit))))
    (Development|PrintString (Utilities|GetDisplayName _asbp_third_person_character))
    (Game|Damage|ApplyDamage (.HitActor (Collision|BreakHitResult _outhit)) 1e+01 0 0)))

(event Custom|PlayAttackMontange
  ;[1 1 1] 적 공격 애니메이션
  (Animation|Montage|PlayMontage (Variables|Character|GetMesh) "/Game/Zombie/Animation/Zombie_Attack_Montage.Zombie_Attack_Montage" 2.0
    (:OnCompleted
      (if (> (Math|Vector|Distance(Vector) (Transformation|GetActorLocation self) (Transformation|GetActorLocation (Variables|Default|GetChaseChar))) 1.5e+02)
        (CallFunction|ChasePlayer)
        (else
          (CallFunction|Attack))))))

(event Custom|SetChar
  ;[1 1 1] 쫓을 플레이어 설정
  (Variables|Default|SetChaseChar (Pawn|GetControlledPawn (Utilities|Array|Get(acopy) (Variables|/Game/Blueprint/GameFrameWork/BP_GM.BP_GM_C|GetAllPlayerControllers (.AsBP%20GM (Utilities|Casting|CastToBP_GM (Game|GetGameMode)))) (Variables|Default|GetChaseIndex)))))

(event Custom|GetDamage
  (params (Damage :type Float%20%28double-precision%29))
  (bind _output_get (Variables|Default|Sethealth (- (Variables|Default|Gethealth) Damage)))
  (if (<= _output_get 0.0)
    (Actor|DestroyActor)))

(event EventBeginPlay
  ;[1 1 1] 쫓을 플레이어 설정
)

(event EventEndPlay
  (params (EndPlayReason :type EEndPlayReason%20Enum :default "Destroyed")))

(fn ConstructionScript)